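; BP_E01_Garde is an enemy guard character with a weapon mesh attached to its left hand socket.
; On BeginPlay it caches its ABP_Guard anim instance and the third-person player character, then attaches the weapon, stopping early if either cast fails.
; MoveCheckSpeed sets walk speed from the EtatGarde state: stationary for Idle and Shoot, slower for Patrol, faster for Chase.
; State changes and calls to MoveCheckSpeed are not made in this graph.
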(event Custom|MoveCheckSpeed
  (switch Utilities|FlowControl|Switch|SwitchonEnum_Garde (Variables|Default|GetEtatGarde)
    (:NewEnumerator0
      (Variables|/Script/Engine.CharacterMovementComponent|SetMaxWalkSpeed (Variables|Character|GetCharacterMovement) 0.0))
    (:NewEnumerator1
      (Variables|/Script/Engine.CharacterMovementComponent|SetMaxWalkSpeed (Variables|Character|GetCharacterMovement) 2e+02))
    (:NewEnumerator2
      (Variables|/Script/Engine.CharacterMovementComponent|SetMaxWalkSpeed (Variables|Character|GetCharacterMovement) 4e+02))
    (:NewEnumerator3
      (Variables|/Script/Engine.CharacterMovementComponent|SetMaxWalkSpeed (Variables|Character|GetCharacterMovement) 0.0))))

(event EventBeginPlay
  (bind _asabp_guard (Utilities|Casting|CastToABP_Guard (Components|SkeletalMesh|GetAnimInstance (Variables|Character|GetMesh))))
  (Variables|Default|SetAnimGuard _asabp_guard)
  (bind _asbp_third_person_character (Utilities|Casting|CastToBP_ThirdPersonCharacter (Game|GetPlayerCharacter 0)))
  (Variables|Default|SetPP _asbp_third_person_character)
  (Transformation|AttachComponentToComponent (Variables|Default|GetMeshWeapon) (Variables|Character|GetMesh) "LeftHandSocket" "SnapToTarget" "KeepRelative" "SnapToTarget" false))

(fn ConstructionScript)