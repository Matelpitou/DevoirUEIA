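; BP_Quest is a quest object with a to-do list that can report to a parent quest through Referent.
; CheckQuest loops over the list and calls FinishTheQuest if IsFinished stays true.
; As written, the test looks inverted: a finished entry clears the flag and an unfinished one stops the loop.
; FinishTheQuest has a valid Referent re-check itself, chaining upward, otherwise it calls OnQuestFinished.
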(event EventBeginPlay)

(event Collision|EventActorBeginOverlap
  (params (OtherActor :type Actor%20Object%20Reference)))

(event EventTick
  (params (DeltaSeconds :type Float%20%28single-precision%29)))

(fn ConstructionScript)

(fn FinishtheQuest
  (bind _referent (Variables|Default|GetReferent))
  (Utilities|IsValid _referent
    (:Is%20Valid
      (CallFunction|CheckQuest _referent))
    (:Is%20Not%20Valid
      (Default|CallOnQuestFinished))))

(fn CheckQuest
  (bind _output_get (LocalVariables|SetTailleTableau (- (Utilities|Array|Length (Variables|Default|GetToDoList)) 1)))
  (Variables|Default|SetIsFinished true)
  (bind _index (Utilities|FlowControl|ForLoopwithBreak 0 _output_get :!label _label)
    (:LoopBody
      (if (Variables|BP_Quest_C|GetIsFinished (Utilities|Array|Get(acopy) (Variables|Default|GetToDoList) _index))
        (Variables|Default|SetIsFinished false)
        (else
          (goto _label Break))))
    (:Completed
      (if (Variables|Default|GetIsFinished)
        (CallFunction|FinishtheQuest)))))