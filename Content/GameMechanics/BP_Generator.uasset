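; Generator puzzle actor where the player places colored batteries into slots to match a solution color sequence.
; On BeginPlay it stores three slot positions and tints an indicator per slot through dynamic materials created in construction.
; Overlapping a slot's box calls CheckBattery, which places, takes or swaps the player's held battery.
; When all slots are filled, VerifColor compares battery colors to the solution and only prints the result.
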(event OnComponentBeginOverlap(Box)
  (params (OverlappedComponent :type Primitive%20Component%20Object%20Reference) (OtherActor :type Actor%20Object%20Reference) (OtherComp :type Primitive%20Component%20Object%20Reference) (OtherBodyIndex :type Integer) (bFromSweep :type Boolean) (SweepResult :type Hit%20Result%20Structure%20%28by%20ref%29))
  (Utilities|Casting|CastToBP_ThirdPersonCharacter OtherActor)
  (CallFunction|CheckBattery))

(event OnComponentBeginOverlap(Box1)
  (params (OverlappedComponent :type Primitive%20Component%20Object%20Reference) (OtherActor :type Actor%20Object%20Reference) (OtherComp :type Primitive%20Component%20Object%20Reference) (OtherBodyIndex :type Integer) (bFromSweep :type Boolean) (SweepResult :type Hit%20Result%20Structure%20%28by%20ref%29))
  (Utilities|Casting|CastToBP_ThirdPersonCharacter OtherActor)
  (CallFunction|CheckBattery 1))

(event OnComponentBeginOverlap(Box2)
  (params (OverlappedComponent :type Primitive%20Component%20Object%20Reference) (OtherActor :type Actor%20Object%20Reference) (OtherComp :type Primitive%20Component%20Object%20Reference) (OtherBodyIndex :type Integer) (bFromSweep :type Boolean) (SweepResult :type Hit%20Result%20Structure%20%28by%20ref%29))
  (Utilities|Casting|CastToBP_ThirdPersonCharacter OtherActor)
  (CallFunction|CheckBattery 2))

(event EventBeginPlay
  (bind _asbp_third_person_character (Utilities|Casting|CastToBP_ThirdPersonCharacter (Game|GetPlayerCharacter 0)))
  (Variables|Default|SetPP _asbp_third_person_character)
  (Utilities|Array|SetArrayElem (Variables|Default|GetPosBattery) 0 (Transformation|GetWorldLocation (Variables|Default|GetEmp)))
  (Utilities|Array|SetArrayElem (Variables|Default|GetPosBattery) 1 (Transformation|GetWorldLocation (Variables|Default|GetEmp1)))
  (Utilities|Array|SetArrayElem (Variables|Default|GetPosBattery) 2 (Transformation|GetWorldLocation (Variables|Default|GetEmp2)))
  (bind _output_get (Default|ChooseColor (Variables|Default|GetTheColor) (Utilities|Array|Get(acopy) (Variables|Default|GetSolutionColor))))
  (Rendering|Material|SetVectorParameterValue (Variables|Default|GetMaterialColor) "AlbedoColor" (Math|Conversions|ToLinearColor(Color) _output_get) :!class /Script/Engine.MaterialInstanceDynamic)
  (bind _output_get_2 (Default|ChooseColor (Variables|Default|GetTheColor) (Utilities|Array|Get(acopy) (Variables|Default|GetSolutionColor) 1)))
  (Rendering|Material|SetVectorParameterValue (Variables|Default|GetMaterialColor1) "AlbedoColor" (Math|Conversions|ToLinearColor(Color) _output_get_2) :!class /Script/Engine.MaterialInstanceDynamic)
  (bind _output_get_3 (Default|ChooseColor (Variables|Default|GetTheColor) (Utilities|Array|Get(acopy) (Variables|Default|GetSolutionColor) 2)))
  (Rendering|Material|SetVectorParameterValue (Variables|Default|GetMaterialColor2) "AlbedoColor" (Math|Conversions|ToLinearColor(Color) _output_get_3) :!class /Script/Engine.MaterialInstanceDynamic))

(fn ConstructionScript
  (bind _returnvalue (Rendering|Material|CreateDynamicMaterialInstance (Variables|Default|GetColor) 0 "/Game/Color/M_Base_Inst.M_Base_Inst" "AlbedoColor" :!class /Script/Engine.PrimitiveComponent))
  (Variables|Default|SetMaterialColor _returnvalue)
  (bind _returnvalue_2 (Rendering|Material|CreateDynamicMaterialInstance (Variables|Default|GetColor1) 0 "/Game/Color/M_Base_Inst.M_Base_Inst" "AlbedoColor" :!class /Script/Engine.PrimitiveComponent))
  (Variables|Default|SetMaterialColor1 _returnvalue_2)
  (bind _returnvalue_3 (Rendering|Material|CreateDynamicMaterialInstance (Variables|Default|GetColor2) 0 "/Game/Color/M_Base_Inst.M_Base_Inst" "AlbedoColor" :!class /Script/Engine.PrimitiveComponent))
  (Variables|Default|SetMaterialColor2 _returnvalue_3))

(fn CheckBattery
  (params (ITableau :type Integer))
  (bind _output_get (LocalVariables|SetITab ITableau))
  (Utilities|IsValid (Utilities|Array|Get(acopy) (Variables|Default|GetTabBattery) _output_get)
    (:Is%20Valid
      (if (== (Utilities|GetClass (Variables|/Game/ThirdPerson/Blueprints/BP_ThirdPersonCharacter.BP_ThirdPersonCharacter_C|GetObjectInHand (Variables|Default|GetPP))) "/Game/GameMechanics/BP_Battery.BP_Battery_C")
        (LocalVariables|SetSaveBattery (Utilities|Array|Get(acopy) (Variables|Default|GetTabBattery) (LocalVariables|GetITab)))
        (Default|Detach (.AsBP%20Battery (Utilities|Casting|CastToBP_Battery (Variables|/Game/ThirdPerson/Blueprints/BP_ThirdPersonCharacter.BP_ThirdPersonCharacter_C|GetObjectInHand (Variables|Default|GetPP)))) false)
        (Utilities|Array|SetArrayElem (Variables|Default|GetTabBattery) (LocalVariables|GetITab) (.AsBP%20Battery (Utilities|Casting|CastToBP_Battery (Variables|/Game/ThirdPerson/Blueprints/BP_ThirdPersonCharacter.BP_ThirdPersonCharacter_C|GetObjectInHand (Variables|Default|GetPP)))))
        (Transformation|SetWorldLocation (Variables|/Game/GameMechanics/BP_Battery.BP_Battery_C|GetDefaultSceneRoot (.AsBP%20Battery (Utilities|Casting|CastToBP_Battery (Variables|/Game/ThirdPerson/Blueprints/BP_ThirdPersonCharacter.BP_ThirdPersonCharacter_C|GetObjectInHand (Variables|Default|GetPP))))) (Utilities|Array|Get(acopy) (Variables|Default|GetPosBattery) (LocalVariables|GetITab)) false false)
        (bind _output_get_2 (Variables|/Game/ThirdPerson/Blueprints/BP_ThirdPersonCharacter.BP_ThirdPersonCharacter_C|SetObjectInHand (Variables|Default|GetPP) (LocalVariables|GetSaveBattery)))
        (Default|Take (.AsBP%20Battery (Utilities|Casting|CastToBP_Battery _output_get_2)))
        (LocalVariables|SetSaveBattery 0)
        (if (== (Variables|Default|GetNbrBatterie) (Utilities|Array|Length (Variables|Default|GetTabBattery))) :!label _label
          (CallFunction|VerifColor))
        (else
          (Utilities|IsValid (Variables|/Game/ThirdPerson/Blueprints/BP_ThirdPersonCharacter.BP_ThirdPersonCharacter_C|GetObjectInHand (Variables|Default|GetPP))
            (:Is%20Valid
              _)
            (:Is%20Not%20Valid
              (bind _output_get_3 (Variables|/Game/ThirdPerson/Blueprints/BP_ThirdPersonCharacter.BP_ThirdPersonCharacter_C|SetObjectInHand (Variables|Default|GetPP) (Utilities|Array|Get(acopy) (Variables|Default|GetTabBattery) (LocalVariables|GetITab))))
              (Class|BPITransportable|Take(Message) _output_get_3)
              (Utilities|Array|SetArrayElem (Variables|Default|GetTabBattery) (LocalVariables|GetITab) 0)
              (Math|Integer|DecrementInt (Variables|Default|GetNbrBatterie)
                (:%20%20
                  _))))))
      (return))
    (:Is%20Not%20Valid
      (if (== (Utilities|GetClass (Variables|/Game/ThirdPerson/Blueprints/BP_ThirdPersonCharacter.BP_ThirdPersonCharacter_C|GetObjectInHand (Variables|Default|GetPP))) "/Game/GameMechanics/BP_Battery.BP_Battery_C")
        (Utilities|Array|SetArrayElem (Variables|Default|GetTabBattery) (LocalVariables|GetITab) (.AsBP%20Battery (Utilities|Casting|CastToBP_Battery (Variables|/Game/ThirdPerson/Blueprints/BP_ThirdPersonCharacter.BP_ThirdPersonCharacter_C|GetObjectInHand (Variables|Default|GetPP)))))
        (Default|Detach (.AsBP%20Battery (Utilities|Casting|CastToBP_Battery (Variables|/Game/ThirdPerson/Blueprints/BP_ThirdPersonCharacter.BP_ThirdPersonCharacter_C|GetObjectInHand (Variables|Default|GetPP)))) true)
        (Transformation|SetWorldLocation (Variables|/Game/GameMechanics/BP_Battery.BP_Battery_C|GetDefaultSceneRoot (.AsBP%20Battery (Utilities|Casting|CastToBP_Battery (Variables|/Game/ThirdPerson/Blueprints/BP_ThirdPersonCharacter.BP_ThirdPersonCharacter_C|GetObjectInHand (Variables|Default|GetPP))))) (Utilities|Array|Get(acopy) (Variables|Default|GetPosBattery) (LocalVariables|GetITab)) false false)
        (Variables|/Game/ThirdPerson/Blueprints/BP_ThirdPersonCharacter.BP_ThirdPersonCharacter_C|SetObjectInHand (Variables|Default|GetPP) 0)
        (Math|Integer|IncrementInt (Variables|Default|GetNbrBatterie)
          (:%20%20
            (goto _label)))))))

(fn VerifColor
  (LocalVariables|SetIsGood? true)
  (bind _index (Utilities|FlowControl|ForLoopwithBreak 0 (- (Utilities|Array|Length (Variables|Default|GetTabBattery)) 1) :!label _label)
    (:LoopBody
      (if (not (Utilities|Enum|Equal(Enum) (Variables|/Game/GameMechanics/BP_Battery.BP_Battery_C|GetColor (Utilities|Array|Get(acopy) (Variables|Default|GetTabBattery) _index)) (Utilities|Array|Get(acopy) (Variables|Default|GetSolutionColor) _index)))
        (LocalVariables|SetIsGood? false)
        (goto _label Break)))
    (:Completed
      (if (LocalVariables|GetIsGood?)
        (Development|PrintString "gg")
        (else
          (Development|PrintString "Noooooooon"))))))

(fn ChangeColor
  (for _index (range 0 (- (Utilities|Array|Length (Variables|Default|GetSolutionColor)) 1))
    (switch Utilities|FlowControl|Switch|SwitchonEnum_ObjectColor (Utilities|Array|Get(acopy) (Variables|Default|GetSolutionColor) _index))))

(fn COmpareColor
  (params (index :type Integer)))