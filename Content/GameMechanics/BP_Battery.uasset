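; BP_Battery is a colored battery the player can pick up, carry on their back and put down.
; A dynamic material on the cylinder gets its albedo color from BPCEmplacement at BeginPlay.
; Take attaches it to the character's Dos component, registers it as ObjectInHand, disables box collision and finishes AssociateQuest.
; Detach drops it at the character's Pose point, unfinishes the quest and restores collision unless blocked.
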(event EventBeginPlay
  (bind _output_get (Default|ChooseColor (Variables|Default|GetBPC_Emplacement) (Variables|Default|GetColor)))
  (Rendering|Material|SetVectorParameterValue (Variables|Default|GetMaterialCylinder) "AlbedoColor" (Math|Conversions|ToLinearColor(Color) _output_get) :!class /Script/Engine.MaterialInstanceDynamic))

(event EventTake
  (Variables|/Game/GameMechanics/BP_Quest.BP_Quest_C|SetIsFinished (Variables|Default|GetAssociateQuest) true)
  (Transformation|AttachComponentToComponent (Variables|/Game/ThirdPerson/Blueprints/BP_ThirdPersonCharacter.BP_ThirdPersonCharacter_C|GetDos (.AsBP%20Third%20Person%20Character (Utilities|Casting|CastToBP_ThirdPersonCharacter (Game|GetPlayerCharacter 0)))) "None" "SnapToTarget" "SnapToTarget" "KeepRelative" true)
  (Development|PrintString "Hello")
  (Variables|/Game/ThirdPerson/Blueprints/BP_ThirdPersonCharacter.BP_ThirdPersonCharacter_C|SetObjectInHand (.AsBP%20Third%20Person%20Character (Utilities|Casting|CastToBP_ThirdPersonCharacter (Game|GetPlayerCharacter 0))) self)
  (Collision|SetCollisionEnabled (Variables|Default|GetBox) "NoCollision"))

(event EventDetach
  (params (BlockColl? :type Boolean))
  (Variables|/Game/GameMechanics/BP_Quest.BP_Quest_C|SetIsFinished (Variables|Default|GetAssociateQuest) false)
  (Transformation|DetachFromActor "KeepRelative" "KeepRelative" "KeepRelative")
  (Transformation|SetWorldLocation (Variables|Default|GetDefaultSceneRoot) (Transformation|GetWorldLocation (Variables|/Game/ThirdPerson/Blueprints/BP_ThirdPersonCharacter.BP_ThirdPersonCharacter_C|GetPose (.AsBP%20Third%20Person%20Character (Utilities|Casting|CastToBP_ThirdPersonCharacter (Game|GetPlayerCharacter 0))))) false false)
  (if (not BlockColl?)
    (Collision|SetCollisionEnabled (Variables|Default|GetBox) "QueryAndPhysics")))

(fn ConstructionScript
  (bind _returnvalue (Rendering|Material|CreateDynamicMaterialInstance (Variables|Default|GetCylinder) 0 "/Game/Color/M_Base_Inst.M_Base_Inst" "None" :!class /Script/Engine.PrimitiveComponent))
  (Variables|Default|SetMaterialCylinder _returnvalue))